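; Springy fork bounce pad that launches the side-scroller character when it overlaps the Box.
; Launch velocity is the actor's up vector multiplied per axis by the character's absolute incoming speed, scaled by Elasticity plus AdditionalForce.
; The launch overrides Z velocity but adds to XY.
; Air control is boosted for half a second, then set to a fixed lower value rather than restored to its prior one.
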(event `self.Box.OnComponentBeginOverlap`
  (params (OverlappedComponent :type "PrimitiveComponent Object Reference") (OtherActor :type "Actor Object Reference") (OtherComp :type "PrimitiveComponent Object Reference") (OtherBodyIndex :type Integer) (bFromSweep :type Boolean) (SweepResult :type "HitResult Structure (by ref)"))
  (bind _elasticity (`self.Elasticity`))
  (bind _additionalforce (`self.AdditionalForce`))
  ;[1 1 1] Bread
  (bind _asside_scroller_character (cast `/Game/SideScrollerBP/Blueprints/SideScrollerCharacter` OtherActor))
  (bind (_returnvalue_x _returnvalue_y _returnvalue_z) (`KismetMathLibrary.BreakVector` (`self.GetVelocity` _asside_scroller_character)))
  ;[1 1 1] Jump/control
  (`Character.LaunchCharacter` _asside_scroller_character (* (`KismetMathLibrary.GetUpVector` (`self.K2_GetActorRotation`)) (`KismetMathLibrary.MakeVector` (+ (* (`KismetMathLibrary.Abs` _returnvalue_x) _elasticity) _additionalforce) (+ (* (`KismetMathLibrary.Abs` _returnvalue_y) _elasticity) _additionalforce) (+ (* (`KismetMathLibrary.Abs` _returnvalue_z) _elasticity) _additionalforce))) false true)
  (bind _charactermovement (`Character.CharacterMovement` _asside_scroller_character))
  (set `CharacterMovementComponent.AirControl` 1.5 _charactermovement)
  (`KismetSystemLibrary.Delay` 0.5)
  (set `CharacterMovementComponent.AirControl` 0.8 _charactermovement))

(fn `UserConstructionScript`)