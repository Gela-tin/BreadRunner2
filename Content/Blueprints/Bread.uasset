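; Bread is a pickup that attaches itself to the side-scroller character on overlap.
; When a SideScrollerCharacter enters the Box, the StaticMesh snaps to the "Bread" socket on the character's mesh, keeping its world scale.
; After a validity check, it destroys the Box, toggles the TextRender's visibility and disables input on the character for the first player controller.
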(event `self.Box.OnComponentBeginOverlap`
  (params (OverlappedComponent :type "PrimitiveComponent Object Reference") (OtherActor :type "Actor Object Reference") (OtherComp :type "PrimitiveComponent Object Reference") (OtherBodyIndex :type Integer) (bFromSweep :type Boolean) (SweepResult :type "HitResult Structure (by ref)"))
  (bind _asside_scroller_character (cast `/Game/SideScrollerBP/Blueprints/SideScrollerCharacter` OtherActor))
  (`SceneComponent.K2_AttachToComponent` (`self.StaticMesh`) (`Character.Mesh` _asside_scroller_character) "Bread" "SnapToTarget" "SnapToTarget" "KeepWorld" true)
  (`/Engine/EditorBlueprintResources/StandardMacros.IsValid` null
    (:`Is Valid`
      (`ActorComponent.K2_DestroyComponent` (`self.Box`))
      (`SceneComponent.ToggleVisibility` (`self.TextRender`) false)
      (`self.DisableInput` _asside_scroller_character (`GameplayStatics.GetPlayerController` 0)))))

(fn `UserConstructionScript`)