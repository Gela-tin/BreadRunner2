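; Butter particle actor that attaches its particle effect to the side-scroller character when something overlaps its box trigger.
; Each overlap toggles the particle's visibility, then a successful character cast snaps it to the mesh's "Lettuce" socket, keeping world scale.
; A validity check, with no input shown, gates destroying the box and unhiding the actor after a short delay.
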(event `self.Box.OnComponentBeginOverlap`
  (params (OverlappedComponent :type "PrimitiveComponent Object Reference") (OtherActor :type "Actor Object Reference") (OtherComp :type "PrimitiveComponent Object Reference") (OtherBodyIndex :type Integer) (bFromSweep :type Boolean) (SweepResult :type "HitResult Structure (by ref)"))
  (`SceneComponent.ToggleVisibility` (`self.ParticleSystem`) false)
  (bind _asside_scroller_character (cast `/Game/SideScrollerBP/Blueprints/SideScrollerCharacter` OtherActor))
  (`SceneComponent.K2_AttachToComponent` (`self.ParticleSystem`) (`Character.Mesh` _asside_scroller_character) "Lettuce" "SnapToTarget" "SnapToTarget" "KeepWorld" true)
  (`/Engine/EditorBlueprintResources/StandardMacros.IsValid` null
    (:`Is Valid`
      (`ActorComponent.K2_DestroyComponent` (`self.Box`))
      (`KismetSystemLibrary.Delay` 1.0)
      (`self.SetActorHiddenInGame` false))))

(fn `UserConstructionScript`)