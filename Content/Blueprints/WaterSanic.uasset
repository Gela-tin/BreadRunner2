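; WaterSanic is a speed boost pickup whose box overlap sharply raises the player character's max walk speed for three seconds.
; For a SideScrollerCharacter, it snaps its mesh and particle effect to the character's sockets, then detaches them and sets the speed to 600.
; A DoOnce re-arms two seconds later.
; The speed change precedes the cast, so other overlapping actors trigger it without restoring speed or re-arming.
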(event `self.Box.OnComponentBeginOverlap`
  (params (OverlappedComponent :type "PrimitiveComponent Object Reference") (OtherActor :type "Actor Object Reference") (OtherComp :type "PrimitiveComponent Object Reference") (OtherBodyIndex :type Integer) (bFromSweep :type Boolean) (SweepResult :type "HitResult Structure (by ref)"))
  (bind _particlesystem (`self.ParticleSystem`))
  (`/Engine/EditorBlueprintResources/StandardMacros.DoOnce` false :!label _label
    (:`Completed`
      (bind _output_get (set `CharacterMovementComponent.MaxWalkSpeed` 10000.0 (`Character.CharacterMovement` (`GameplayStatics.GetPlayerCharacter` 0))))
      (`KismetSystemLibrary.PrintString` (`KismetStringLibrary.Conv_DoubleToString` _output_get))
      (bind _asside_scroller_character (cast `/Game/SideScrollerBP/Blueprints/SideScrollerCharacter` OtherActor))
      (bind _mesh (`Character.Mesh` _asside_scroller_character))
      (`SceneComponent.K2_AttachToComponent` (`self.StaticMesh`) _mesh "Speed" "SnapToTarget" "SnapToTarget" "SnapToTarget" true)
      (`SceneComponent.K2_AttachToComponent` (`self.ParticleSystem`) _mesh "SpeedParticle" "SnapToTarget" "SnapToTarget" "SnapToTarget" true)
      (`SceneComponent.SetVisibility` _particlesystem true false)
      (`KismetSystemLibrary.Delay` 3.0)
      (`SceneComponent.SetVisibility` _particlesystem false false)
      (`SceneComponent.K2_DetachFromComponent` (`self.ParticleSystem`) "KeepRelative" "KeepRelative" "KeepRelative" true)
      (`SceneComponent.K2_DetachFromComponent` (`self.StaticMesh`) "KeepRelative" "KeepRelative" "KeepRelative" true)
      (bind _output_get_2 (set `CharacterMovementComponent.MaxWalkSpeed` 600.0 (`Character.CharacterMovement` (`GameplayStatics.GetPlayerCharacter` 0))))
      (`KismetSystemLibrary.PrintString` (`KismetStringLibrary.Conv_DoubleToString` _output_get_2))
      (`KismetSystemLibrary.Delay` 2.0)
      (goto _label :!via `Reset`))))

(fn `UserConstructionScript`)