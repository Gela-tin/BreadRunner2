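; Slippery butter hazard for the side-scroller that sends the player sliding along +Y when a SideScrollerCharacter overlaps its box.
; On overlap it launches player 0, destroys its own mesh and box, forces movement input and plays the slide animation.
; It zeroes velocity, ground friction and braking and disables input, then after a one-second delay restores input and hardcoded friction and braking values.
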(event `self.Box.OnComponentBeginOverlap`
  (params (OverlappedComponent :type "PrimitiveComponent Object Reference") (OtherActor :type "Actor Object Reference") (OtherComp :type "PrimitiveComponent Object Reference") (OtherBodyIndex :type Integer) (bFromSweep :type Boolean) (SweepResult :type "HitResult Structure (by ref)"))
  (bind _returnvalue (`GameplayStatics.GetPlayerCharacter` 0))
  (bind _charactermovement (`Character.CharacterMovement` _returnvalue))
  (bind _asside_scroller_character (cast `/Game/SideScrollerBP/Blueprints/SideScrollerCharacter` OtherActor))
  (`Character.LaunchCharacter` _returnvalue (0.0 1000.0 0.0) false false)
  (`ActorComponent.K2_DestroyComponent` (`self.StaticMesh`))
  (`ActorComponent.K2_DestroyComponent` (`self.Box`))
  (`Pawn.AddMovementInput` _asside_scroller_character (0.0 300.0 0.0) 10.0 true)
  (`SkeletalMeshComponent.PlayAnimation` (`Character.Mesh` _returnvalue) "/Game/Bread/Running_Slide.Running_Slide" false)
  (set `CharacterMovementComponent.GroundFriction` 0.0 _charactermovement)
  (set `CharacterMovementComponent.BrakingDecelerationWalking` 0.0 _charactermovement)
  (set `CharacterMovementComponent.BrakingFrictionFactor` 0.0 _charactermovement)
  (set `MovementComponent.Velocity` (0.0 0.0 0.0) _charactermovement)
  (`self.DisableInput` _returnvalue null)
  (`KismetSystemLibrary.Delay` 1.0)
  (`self.EnableInput` _returnvalue null)
  (set `CharacterMovementComponent.GroundFriction` 3.0 _charactermovement)
  (set `CharacterMovementComponent.BrakingDecelerationWalking` 2048.0 _charactermovement)
  (set `CharacterMovementComponent.BrakingFrictionFactor` 2.0 _charactermovement))

(fn `UserConstructionScript`)